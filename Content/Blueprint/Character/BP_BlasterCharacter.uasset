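; BP_BlasterCharacter is the character Blueprint that handles the overhead name display and sniper scope overlay.
; On BeginPlay it passes itself to WBP_OverheadWidget to show the player name.
; ShowSniperScopeWidget lazily creates and caches WBP_SniperScope, then plays one zoom animation forward or reversed with matching zoom sounds.
; Escape quits the game, and an unconnected ShowPlayerNetRole call never runs.
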(event EventBeginPlay
  (bind _aswbp_overhead_widget (Utilities|Casting|CastToWBP_OverheadWidget (UserInterface|GetUserWidgetObject (Variables|Default|GetOverheadWidget))))
  (Class|OverheadWidget|ShowPlayerName _aswbp_overhead_widget self))

(event Collision|EventActorBeginOverlap
  (params (OtherActor :type Actor%20Object%20Reference)))

(event EventTick
  (params (DeltaSeconds :type Float%20%28single-precision%29)))

(event EventShowSniperScopeWidget
  (params (bShowScope :type Boolean))
  (Utilities|IsValid (Variables|Default|GetSniperScopeWidget)
    (:Is%20Valid
      _)
    (:Is%20Not%20Valid
      (bind _returnvalue (UserInterface|CreateWidget "/Game/Blueprint/HUD/WBP_SniperScope.WBP_SniperScope_C"))
      (bind _output_get (Variables|Default|SetSniperScopeWidget _returnvalue))
      (UserInterface|Viewport|AddtoViewport _output_get 0)))
  (if bShowScope
    (bind _sniperscopewidget (Variables|Default|GetSniperScopeWidget)
      (:then
        (UserInterface|Animation|PlayAnimation _sniperscopewidget (Variables|/Game/Blueprint/HUD/WBP_SniperScope.WBP_SniperScope_C|GetScopeZoomIn _sniperscopewidget) 0.0 1 "Forward" 1.0 false)
        (Audio|PlaySound2D "/Game/Assets/MilitaryWeapSilver/Sound/SniperRifle/Cues/SniperRifle_ZoomIn_Cue.SniperRifle_ZoomIn_Cue" 1.0 1.0 0.0 0 0))
      (:else))
    (else
      (bind _sniperscopewidget_2 (Variables|Default|GetSniperScopeWidget)
        (:then
          (UserInterface|Animation|PlayAnimation _sniperscopewidget_2 (Variables|/Game/Blueprint/HUD/WBP_SniperScope.WBP_SniperScope_C|GetScopeZoomIn _sniperscopewidget_2) 0.0 1 "Reverse" 1.0 false)
          (Audio|PlaySound2D "/Game/Assets/MilitaryWeapSilver/Sound/SniperRifle/Cues/SniperRifle_ZoomOut_Cue.SniperRifle_ZoomOut_Cue" 1.0 1.0 0.0 0 0))
        (:else)))))

(event Input|KeyboardEvents|Escape
  (params (Key :type Key%20Structure :default "None"))
  (:Pressed
    (Game|QuitGame 0 "Quit" false)))

(fn ConstructionScript)